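; Game mode for a Frogger-style game that runs the attempt loop, scoring and game over.
; Each attempt spawns a frog, camera and audio listener, with timers driving the ticking warning and time limit.
; Frog death and home-arrival events award points or deduct attempts, then respawn or show a win or lose screen.
; Running out of time on the last attempt shows the win screen, unlike death.
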(event `self.ReceiveBeginPlay`
  (`/Game/Blueprints/BP_UILibrary.CreateWidget` self "/Game/Blueprints/Widgets/WBP_MainMenu.WBP_MainMenu_C" true true true)
  (bind _outactors (`GameplayStatics.GetAllActorsOfClass` "/Game/Blueprints/BP_FrogHome.BP_FrogHome_C"))
  (set `self.HomeCount` (`KismetArrayLibrary.Array_Length` _outactors))
  (set `self.CurrentScore` 0))

(event `OnPlay`
  (`WidgetBlueprintLibrary.SetInputMode_UIOnlyEx` (`GameplayStatics.GetPlayerController` 0) null)
  (`KismetSystemLibrary.K2_SetTimerDelegate` (delegate `OnStartGame`) 1.0)
  (`self.CreatePlayer`))

(event `OnStartGame`
  (bind _returnvalue (`KismetSystemLibrary.K2_SetTimerDelegate` (`|CreateDelegate` :!event `OnTimerNearDone`) (- (`self.TimeLimitPerAttempt`) 10.0)))
  (set `self.TimeTickHandler` _returnvalue)
  (bind _returnvalue_2 (`KismetSystemLibrary.K2_SetTimerDelegate` (`|CreateDelegate` :!event `OnTimeLimitReached`) (`self.TimeLimitPerAttempt`)))
  (set `self.AttemptTimeHandler` _returnvalue_2)
  (`WidgetBlueprintLibrary.SetInputMode_GameOnly` (`GameplayStatics.GetPlayerController` 0))
  (bind _foundwidgets (`WidgetBlueprintLibrary.GetAllWidgetsOfClass` "/Game/Blueprints/Widgets/WBP_GameUI.WBP_GameUI_C"))
  (for _array_element _foundwidgets
    (`Widget.SetVisibility` (`/Game/Blueprints/Widgets/WBP_GameUI.AttemptTimer` _array_element) "Visible")))

(event `OnFrogArrivedHome`
  (`KismetSystemLibrary.K2_PauseTimerHandle` (`self.AttemptTimeHandler`))
  (`self.StopTimerSound`)
  (`self.AddScore` "NewEnumerator1")
  (`self.AddScore` "NewEnumerator3")
  (`self.DisablePlayerInput`
    (:`Out`
      (`KismetSystemLibrary.Delay` 1.0)
      (`self.DestroyPlayer` false)
      (`/Engine/EditorBlueprintResources/StandardMacros.IncrementInt` (`self.HomesReached`)
        (:`  `
          (bind _result (`self.AreAllHomesReached`))
          (if _result
            (`self.AddScore` "NewEnumerator2")
            (`self.AddScore` "NewEnumerator4")
            (`self.OnGameOver` true)
            (else
              (`self.OnPlay`))))))))

(event `OnPlayerDeath`
  (`KismetSystemLibrary.K2_PauseTimerHandle` (`self.AttemptTimeHandler`))
  (`self.StopTimerSound`)
  (`GameplayStatics.PlaySound2D` "/Game/Audio/Jingles/S_Jingle_Death.S_Jingle_Death" 0.8 1.0 0.0 null null false)
  (`KismetSystemLibrary.Delay` 1.0)
  (`self.DestroyPlayer` true)
  (if (== (`self.AttemptsRemaining`) 0)
    (`self.OnGameOver` false)
    (else
      (`self.DeductAttempts`)
      (`self.OnPlay`))))

(event `OnTimerNearDone`
  (`self.PlayTimerSound` "/Game/Audio/Timer/S_Timer_Tick_Cue.S_Timer_Tick_Cue"))

(event `OnTimeLimitReached`
  (`KismetSystemLibrary.K2_PauseTimerHandle` (`self.AttemptTimeHandler`))
  (`self.PlayTimerSound` "/Game/Audio/Timer/S_Timer_Ding_Cue.S_Timer_Ding_Cue")
  (if (== (`self.AttemptsRemaining`) 0)
    (`self.OnGameOver` true)
    (else
      (`self.DestroyPlayer` true)
      (`self.DeductAttempts`)
      (`self.OnPlay`))))

(event `OnGameOver`
  (params (ShowFinalScore :type Boolean))
  (`KismetSystemLibrary.K2_PauseTimerHandle` (`self.TimeTickHandler`))
  (if ShowFinalScore
    (`/Game/Blueprints/BP_UILibrary.CreateWidget` self "/Game/Blueprints/Widgets/WBP_WinScreen.WBP_WinScreen_C" true true true)
    (`GameplayStatics.PlaySound2D` "/Game/Audio/Jingles/S_Jingle_Game_Over_Win.S_Jingle_Game_Over_Win" 1.0 1.0 0.0 null null false)
    (else
      (`/Game/Blueprints/BP_UILibrary.CreateWidget` self "/Game/Blueprints/Widgets/WBP_LoseScreen.WBP_LoseScreen_C" true true true)
      (`GameplayStatics.PlaySound2D` "/Game/Audio/Jingles/S_Jingle_Game_Over_Lose.S_Jingle_Game_Over_Lose" 1.0 1.0 0.0 null null false))))

(fn `AddScore`
  (params (ScoreCategory :type "/Game/Data/E_ScoreCategory Enum" :default "NewEnumerator0"))
  (switch `/Game/Data/E_ScoreCategory` ScoreCategory
    (:`NewEnumerator0`
      (`self.AddScoreDirectly` (`self.Score_StepForward`)))
    (:`NewEnumerator1`
      (`self.AddScoreDirectly` (`self.Score_ArrivedHome`)))
    (:`NewEnumerator2`
      (`self.AddScoreDirectly` (`self.Score_AllArrivedHome`)))
    (:`NewEnumerator3`
      (bind _time (`self.GetTimeRemaining`))
      (`self.AddScoreMultiplier` (`self.Score_PerSecondTimeLimit`) _time))
    (:`NewEnumerator4`
      (`self.AddScoreMultiplier` (`self.Score_AttemptsRemaining`) (`self.AttemptsRemaining`)))))

(fn `AreAllHomesReached`
  (returns (Result :type Boolean))
  (return (== (`self.HomesReached`) (`self.HomeCount`))))

(fn `CreatePlayer`
  (bind _returnvalue (`|SpawnActorFromClass` "/Game/Blueprints/Animals/BP_Frog.BP_Frog_C" (`KismetMathLibrary.MakeTransform` (0.0 0.0 0.0)) "Undefined" "OverrideRootScale" null null))
  (bind _output_get (set `self.Frog` _returnvalue))
  (add `/Game/Blueprints/Animals/BP_Frog.OnDeath` _output_get (`|CreateDelegate` :!event `OnPlayerDeath`))
  (add `/Game/Blueprints/Animals/BP_Frog.OnArrivedHome` _output_get (`|CreateDelegate` :!event `OnFrogArrivedHome`))
  (bind _returnvalue_2 (`|SpawnActorFromClass` "/Game/Blueprints/BP_FrogCamera.BP_FrogCamera_C" (`KismetMathLibrary.MakeTransform` (0.0 0.0 0.0)) "Undefined" "OverrideRootScale" null null))
  (set `/Game/Blueprints/BP_FrogCamera.Frog` (`self.Frog`) _returnvalue_2)
  (bind _returnvalue_3 (`|SpawnActorFromClass` "/Game/Blueprints/BP_AudioListener.BP_AudioListener_C" (`KismetMathLibrary.MakeTransform` (0.0 0.0 0.0)) "Undefined" "OverrideRootScale" null null))
  (bind _output_get_2 (set `self.AudioListener` _returnvalue_3))
  (set `/Game/Blueprints/BP_AudioListener.Target` (`self.Frog`) _output_get_2))

(fn `DeductAttempts`
  (`/Engine/EditorBlueprintResources/StandardMacros.DecrementInt` (`self.AttemptsRemaining`)
    (:`  `
      (`self.OnDeductAttempt`))))

(fn `DestroyPlayer`
  (params (DestroyPlayer :type Boolean :default true) (DestroyCamera :type Boolean :default true))
  (bind _frog (`self.Frog`))
  (if DestroyPlayer
    (`self.K2_DestroyActor` _frog)
    (else
      (`self.DisableInput` _frog (`GameplayStatics.GetPlayerController` 0))))
  (`self.K2_DestroyActor` (`self.AudioListener`))
  (if (`local.DestroyCamera`)
    (bind _returnvalue (`GameplayStatics.GetActorOfClass` "/Game/Blueprints/BP_FrogCamera.BP_FrogCamera_C"))
    (`self.K2_DestroyActor` _returnvalue)))

(fn `GetPercentOutOfBounds`
  (params (Point :type "Vector Structure"))
  (returns (Value :type "Float (double-precision)"))
  (bind _returnvalue (`KismetMathLibrary.Abs` (`KismetMathLibrary.FMin` (`self.LeftLevelBound`) (`self.RightLevelBound`))))
  (return (/ (- (`KismetMathLibrary.Abs` (.y Point)) _returnvalue) (- (`KismetMathLibrary.Abs` (`KismetMathLibrary.FMin` (`self.LeftSpawnBound`) (`self.RightSpawnBound`))) _returnvalue))))

(fn `GetTimeRemaining`
  (returns (Time :type Integer))
  (return (`KismetMathLibrary.FFloor` (`KismetSystemLibrary.K2_GetTimerRemainingTimeHandle` (`self.AttemptTimeHandler`)))))

(fn `IsPointInsideLevelBound`
  (params (Point :type "Vector Structure"))
  (returns (Result :type Boolean))
  (bind (_x _y) (`KismetMathLibrary.BreakVector3f` Point))
  (return (and (< _x (`self.UpperLevelBound`)) (> _x (`self.LowerLevelBound`)) (> _y (`self.LeftLevelBound`)) (< _y (`self.RightLevelBound`)))))

(fn `PlayTimerSound`
  (params (Sound :type "SoundBase Object Reference"))
  (bind _timer (`self.Timer`))
  (`self.StopTimerSound`)
  (`AudioComponent.SetSound` _timer Sound)
  (`AudioComponent.Play` _timer 0.0))

(fn `StopTimerSound`
  (`AudioComponent.Stop` (`self.Timer`)))

(fn `UserConstructionScript`)