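; Player-controlled frog for a Frogger-style game, hopping across a grid in four directions.
; Input rotates the frog, flags the anim blueprint and plays a timeline that lerps it one GameMode GridSpacing step forward, blocking new moves until finished.
; Sphere overlaps trigger death on DeathBox-tagged components, report arrival at BP_FrogHome, or lock the frog each tick to a climbable platform's nearest spot until overlap ends.
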(event `self.ReceiveBeginPlay`
  (bind _asabp_frog (cast `/Game/Blueprints/Animals/ABP_Frog` (`SkeletalMeshComponent.GetAnimInstance` (`self.SK_Frog`))))
  (set `self.AnimationBlueprint` _asabp_frog)
  (set `self.LastPosition` (`self.K2_GetActorLocation`))
  (`TimelineComponent.SetPlayRate` (`self.MoveTimeline`) 6.5)
  (bind _returnvalue (`GameplayStatics.GetActorOfClass` "/Game/Blueprints/BP_FroggyRoadGameMode.BP_FroggyRoadGameMode_C"))
  (set `self.MoveStepSize` (`/Game/Blueprints/BP_FroggyRoadGameMode.GridSpacing` _returnvalue)))

(event `self.ReceiveTick`
  (params (DeltaSeconds :type "Float (single-precision)"))
  (if (`self.IsClimbing`)
    (`self.K2_SetActorLocation` (`SceneComponent.K2_GetComponentLocation` (`self.ClimbSpot`)) true)))

(event `InputAction|Up`
  (params (Key :type "Key Structure"))
  (:`Pressed`
    (if (`self.CanMove`)
      (set `/Game/Blueprints/Animals/ABP_Frog.IsJumping` true (`self.AnimationBlueprint`))
      (`self.SetDirection` "NewEnumerator0")
      (set `self.StartedMoving` true :!label _label)
      (set `self.LastPosition` (`self.K2_GetActorLocation`))
      (set `self.NextPosition` (+ (`self.LastPosition`) (* (`self.GetActorForwardVector`) (`KismetMathLibrary.Conv_DoubleToVector` (`self.MoveStepSize`)))))
      (`self.OnMove`))))

(event `InputAction|Down`
  (params (Key :type "Key Structure"))
  (:`Pressed`
    (if (`self.CanMove`)
      (set `/Game/Blueprints/Animals/ABP_Frog.IsJumping` true (`self.AnimationBlueprint`))
      (`self.SetDirection` "NewEnumerator1")
      (goto _label))))

(event `InputAction|Left`
  (params (Key :type "Key Structure"))
  (:`Pressed`
    (if (`self.CanMove`)
      (set `/Game/Blueprints/Animals/ABP_Frog.IsJumping` true (`self.AnimationBlueprint`))
      (`self.SetDirection` "NewEnumerator2")
      (goto _label))))

(event `InputAction|Right`
  (params (Key :type "Key Structure"))
  (:`Pressed`
    (if (`self.CanMove`)
      (set `/Game/Blueprints/Animals/ABP_Frog.IsJumping` true (`self.AnimationBlueprint`))
      (`self.SetDirection` "NewEnumerator3")
      (goto _label))))

(event `OnMove`
  (if (`self.StartedMoving`)
    (set `self.StartedMoving` false)
    (set `self.CanMove` false)
    (bind (_direction _alpha) (`Timeline|MoveTimeline` :!via `PlayFromStart`)
      (:`Update`
        (`self.Move` _alpha))
      (:`Finished`
        (set `self.CanMove` true)))))

(event `self.Sphere.OnComponentBeginOverlap`
  (params (OverlappedComponent :type "PrimitiveComponent Object Reference") (OtherActor :type "Actor Object Reference") (OtherComp :type "PrimitiveComponent Object Reference") (OtherBodyIndex :type Integer) (bFromSweep :type Boolean) (SweepResult :type "HitResult Structure (by ref)"))
  (if (`ActorComponent.ComponentHasTag` OtherComp "DeathBox")
    (set `/Game/Blueprints/Animals/ABP_Frog.IsDead` true (`self.AnimationBlueprint`))
    (`ActorComponent.K2_DestroyComponent` (`self.Sphere`))
    (`WidgetBlueprintLibrary.SetInputMode_UIOnlyEx` (`GameplayStatics.GetPlayerController` 0) null)
    (`self.OnDeath`)
    (else
      (bind _asbp_climbable_platform_item (cast `/Game/Blueprints/BP_ClimbablePlatformItem` OtherActor)
        (:`then`
          (set `self.IsClimbing` true)
          (bind _spot (`/Game/Blueprints/BP_ClimbablePlatformItem.GetNearestClimbSpot` _asbp_climbable_platform_item (`self.K2_GetActorLocation`)))
          (set `self.ClimbSpot` _spot))
        (:`CastFailed`
          (cast `/Game/Blueprints/BP_FrogHome` OtherActor)
          (`self.OnArrivedHome`))))))

(event `self.Sphere.OnComponentEndOverlap`
  (params (OverlappedComponent :type "PrimitiveComponent Object Reference") (OtherActor :type "Actor Object Reference") (OtherComp :type "PrimitiveComponent Object Reference") (OtherBodyIndex :type Integer))
  (cast `/Game/Blueprints/BP_ClimbablePlatformItem` OtherActor)
  (set `self.IsClimbing` false))

(fn `GetDirectionVectorAndRotator`
  (params (Direction :type "/Game/Data/E_FrogDirection Enum" :default "NewEnumerator0"))
  (returns (Vector :type "Vector Structure") (Rotator :type "Rotator Structure"))
  (switch `/Game/Data/E_FrogDirection` Direction
    (:`NewEnumerator0`
      (bind (_vector _rotator) (`/Game/Blueprints/BP_TransformUtility.GetForwardVectorAndRotator`))
      (return _vector _rotator))
    (:`NewEnumerator1`
      (bind (_vector_2 _rotator_2) (`/Game/Blueprints/BP_TransformUtility.GetBackwardVectorAndRotator`))
      (return _vector_2 _rotator_2))
    (:`NewEnumerator2`
      (bind (_vector_3 _rotator_3) (`/Game/Blueprints/BP_TransformUtility.GetLeftVectorAndRotator`))
      (return _vector_3 _rotator_3))
    (:`NewEnumerator3`
      (bind (_vector_4 _rotator_4) (`/Game/Blueprints/BP_TransformUtility.GetRightVectorAndRotator`))
      (return _vector_4 _rotator_4))))

(fn `Move`
  (params (Alpha :type "Float (double-precision)"))
  (`self.K2_SetActorLocation` (`KismetMathLibrary.VLerp` (`self.LastPosition`) (`self.NextPosition`) Alpha) true))

(fn `SetDirection`
  (params (Direction :type "/Game/Data/E_FrogDirection Enum" :default "NewEnumerator0"))
  (bind (_vector _rotator) (`self.GetDirectionVectorAndRotator` Direction))
  (`self.K2_SetActorRotation` _rotator))

(fn `UserConstructionScript`)