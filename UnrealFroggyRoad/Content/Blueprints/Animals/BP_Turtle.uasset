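; BP_Turtle is a turtle actor that reacts when a frog climbs onto it.
; On BeginPlay it randomly marks itself as a sinker, with a small chance.
; When ClimberDetector overlaps a BP_Frog, it plays a shell impact sound and activates its Ripple effect.
; If it is a sinker, the overlap also sets DirectionModifier to point downward, presumably making it sink.
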(event `self.ReceiveBeginPlay`
  (`parent.ReceiveBeginPlay`)
  (set `self.IsSinking` (`KismetMathLibrary.RandomBoolWithWeight` 0.05)))

(event `self.ClimberDetector.OnComponentBeginOverlap`
  (params (OverlappedComponent :type "PrimitiveComponent Object Reference") (OtherActor :type "Actor Object Reference") (OtherComp :type "PrimitiveComponent Object Reference") (OtherBodyIndex :type Integer) (bFromSweep :type Boolean) (SweepResult :type "HitResult Structure (by ref)"))
  (cast `/Game/Blueprints/Animals/BP_Frog` OtherActor)
  (`GameplayStatics.PlaySound2D` "/Game/Audio/Impact/S_Shell_Impact.S_Shell_Impact" 1.0 1.0 0.0 null null false)
  (`ActorComponent.Activate` (`self.Ripple`) true)
  (if (`self.IsSinking`)
    (set `self.DirectionModifier` (0.0 0.0 -100.0))))

(fn `UserConstructionScript`)