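; BP_PlatformItem is an actor that travels along its forward vector while IsMoving is set and destroys itself past a kill boundary.
; BeginPlay maps the Speed setting to MoveSpeed across four tiers, from Very Slow to Fast.
; Tick sweeps the root by a delta-time-scaled forward step plus an unscaled DirectionModifier, so that offset is frame-rate dependent.
; The kill check compares absolute world Y against KillBoundY, making it symmetric around zero.
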(event `self.ReceiveBeginPlay`
  (switch `/Game/Data/E_PlatformItemSpeed` (`self.Speed`)
    (:`NewEnumerator3`
      (set `self.MoveSpeed` 500.0))
    (:`NewEnumerator0`
      (set `self.MoveSpeed` 800.0))
    (:`NewEnumerator1`
      (set `self.MoveSpeed` 1200.0))
    (:`NewEnumerator2`
      (set `self.MoveSpeed` 1600.0))))

(event `self.ReceiveTick`
  (params (DeltaSeconds :type "Float (single-precision)"))
  (if (`self.IsMoving`)
    (`SceneComponent.K2_AddRelativeLocation` (`self.DefaultSceneRoot`) (+ (* DeltaSeconds (`self.MoveSpeed`) (`self.GetActorForwardVector`)) (`self.DirectionModifier`)) true false)
    (if (> (`KismetMathLibrary.Abs` (`.Y` (`KismetMathLibrary.BreakVector3f` (`self.K2_GetActorLocation`)))) (`KismetMathLibrary.Abs` (`self.KillBoundY`)))
      (`self.K2_DestroyActor`))))

(fn `UserConstructionScript`)