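; Player-controlled frog that hops in fixed steps along the four world axes, one hop at a time.
; Directional input snaps its rotation, flags the jump on its Animation Blueprint and targets a point one step ahead.
; A timeline lerps it there with a swept move, blocking input until the hop finishes.
; Tick draws debug arrows for frog and world forward vectors plus last and next positions.
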(event `self.ReceiveBeginPlay`
  (bind _asabp_frog (cast `/Game/Blueprints/ABP_Frog` (`SkeletalMeshComponent.GetAnimInstance` (`self.SK_Frog`))))
  (set `self.AnimationBlueprint` _asabp_frog)
  (set `self.LastPosition` (`self.K2_GetActorLocation`))
  (`TimelineComponent.SetPlayRate` (`self.MoveTimeline`) 5.0))

(event `self.ReceiveTick`
  (params (DeltaSeconds :type "Float (single-precision)"))
  (`self.DrawDebugForwardVectors`
    (:`Out`
      (`self.DrawDebugLastPosition`
        (:`Out`
          (`self.DrawDebugNextPosition`))))))

(event `InputAction|Up`
  (params (Key :type "Key Structure"))
  (:`Pressed`
    (if (`self.CanMove`)
      (set `/Game/Blueprints/ABP_Frog.IsJumping` true (`self.AnimationBlueprint`))
      (`self.SetDirection` "NewEnumerator0")
      (if (not (`self.IsMoving`)) :!label _label
        (set `self.StartedMoving` true)
        (bind _output_get (set `self.IsMoving` true))
        (if _output_get
          (`self.OnMove`)
          (set `self.NextPosition` (+ (`self.LastPosition`) (* (`self.GetActorForwardVector`) (`KismetMathLibrary.Conv_DoubleToVector` (`self.MoveStepSize`))))))))))

(event `InputAction|Down`
  (params (Key :type "Key Structure"))
  (:`Pressed`
    (if (`self.CanMove`)
      (set `/Game/Blueprints/ABP_Frog.IsJumping` true (`self.AnimationBlueprint`))
      (`self.SetDirection` "NewEnumerator1")
      (goto _label))))

(event `InputAction|Left`
  (params (Key :type "Key Structure"))
  (:`Pressed`
    (if (`self.CanMove`)
      (set `/Game/Blueprints/ABP_Frog.IsJumping` true (`self.AnimationBlueprint`))
      (`self.SetDirection` "NewEnumerator2")
      (goto _label))))

(event `InputAction|Right`
  (params (Key :type "Key Structure"))
  (:`Pressed`
    (if (`self.CanMove`)
      (set `/Game/Blueprints/ABP_Frog.IsJumping` true (`self.AnimationBlueprint`))
      (`self.SetDirection` "NewEnumerator3")
      (goto _label))))

(event `OnMove`
  (if (`self.StartedMoving`)
    (set `self.StartedMoving` false)
    (set `self.CanMove` false)
    (bind (_direction _alpha) (`Timeline|MoveTimeline` :!via `PlayFromStart` :!label _label_2)
      (:`Update`
        (`self.Move` _alpha))
      (:`Finished`
        (set `self.IsMoving` false)
        (set `self.CanMove` true)
        (set `self.LastPosition` (`self.K2_GetActorLocation`))))
    (else
      (goto _label_2))))

(fn `GetDirectionVectorAndRotator`
  (params (Direction :type "/Game/Blueprints/E_FrogDirection Enum" :default "NewEnumerator0"))
  (returns (Vector :type "Vector Structure") (Rotator :type "Rotator Structure"))
  (bind _returnvalue (`KismetMathLibrary.GetForwardVector` (struct)))
  (bind _returnvalue_2 (`KismetMathLibrary.GetRightVector` (struct)))
  (bind _returnvalue_3 (`KismetMathLibrary.NegateVector` (`KismetMathLibrary.GetForwardVector` (struct))))
  (bind _returnvalue_4 (`KismetMathLibrary.NegateVector` (`KismetMathLibrary.GetRightVector` (struct))))
  (switch `/Game/Blueprints/E_FrogDirection` Direction
    (:`NewEnumerator0`
      (return _returnvalue (`KismetMathLibrary.Conv_VectorToRotator` _returnvalue)))
    (:`NewEnumerator1`
      (return _returnvalue_3 (`KismetMathLibrary.Conv_VectorToRotator` _returnvalue_3)))
    (:`NewEnumerator2`
      (return _returnvalue_4 (`KismetMathLibrary.Conv_VectorToRotator` _returnvalue_4)))
    (:`NewEnumerator3`
      (return _returnvalue_2 (`KismetMathLibrary.Conv_VectorToRotator` _returnvalue_2)))))

(fn `Move`
  (params (Alpha :type "Float (double-precision)"))
  (`self.K2_SetActorLocation` (`KismetMathLibrary.VLerp` (`self.LastPosition`) (`self.NextPosition`) Alpha) true))

(fn `SetDirection`
  (params (Direction :type "/Game/Blueprints/E_FrogDirection Enum" :default "NewEnumerator0"))
  (bind (_vector _rotator) (`self.GetDirectionVectorAndRotator` Direction))
  (`self.K2_SetActorRotation` _rotator))

(fn `UserConstructionScript`)