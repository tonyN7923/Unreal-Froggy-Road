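; BP_LevelBoundVolume is a box volume marking an out-of-bounds area for the frog player.
; When BP_Frog enters the box, it caches the frog and BP_FrogCamera, flags the player as out of bounds and plays a warning jingle.
; While flagged, Tick passes the frog's location to the camera's FadeOutOfBounds every frame.
; Leaving the box sets the in-bound flag, which stops those calls.
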(event `self.ReceiveTick`
  (params (DeltaSeconds :type "Float (single-precision)"))
  (if (not (`self.IsPlayerInBound`))
    (`/Game/Blueprints/BP_FrogCamera.FadeOutOfBounds` (`self.FrogCamera`) (`self.K2_GetActorLocation` (`self.Frog`)))))

(event `self.Box.OnComponentBeginOverlap`
  (params (OverlappedComponent :type "PrimitiveComponent Object Reference") (OtherActor :type "Actor Object Reference") (OtherComp :type "PrimitiveComponent Object Reference") (OtherBodyIndex :type Integer) (bFromSweep :type Boolean) (SweepResult :type "HitResult Structure (by ref)"))
  (bind _asbp_frog (cast `/Game/Blueprints/Animals/BP_Frog` OtherActor))
  (set `self.Frog` _asbp_frog)
  (bind _returnvalue (`GameplayStatics.GetActorOfClass` "/Game/Blueprints/BP_FrogCamera.BP_FrogCamera_C"))
  (set `self.FrogCamera` _returnvalue)
  (set `self.IsPlayerInBound` false)
  (`GameplayStatics.PlaySound2D` "/Game/Audio/Jingles/S_Jingle_OutOfBound.S_Jingle_OutOfBound" 0.8 1.0 0.0 null null false))

(event `self.Box.OnComponentEndOverlap`
  (params (OverlappedComponent :type "PrimitiveComponent Object Reference") (OtherActor :type "Actor Object Reference") (OtherComp :type "PrimitiveComponent Object Reference") (OtherBodyIndex :type Integer))
  (cast `/Game/Blueprints/Animals/BP_Frog` OtherActor)
  (`GameplayStatics.GetActorOfClass` "/Game/Blueprints/BP_FrogCamera.BP_FrogCamera_C")
  (set `self.IsPlayerInBound` true))

(fn `UserConstructionScript`)