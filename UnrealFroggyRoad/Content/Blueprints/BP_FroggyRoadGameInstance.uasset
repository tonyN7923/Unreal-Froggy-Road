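; Game instance for Froggy Road that owns the persistent audio settings and high score saves.
; On init it loads both save objects, creating new ones when no slot exists, then after a short delay applies the saved volumes.
; Volumes are applied as per-class overrides on a master sound mix, covering master, music, environment, SFX and UI.
; Save functions write each object back to its slot.
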(event `self.ReceiveInit`
  (`self.LoadAllSaves`)
  (`KismetSystemLibrary.Delay` 0.1)
  (`self.InitializeVolumes`))

(fn `InitializeVolumes`
  (bind _savegame_audiosettings (`self.SaveGame_AudioSettings`))
  (`self.SetVolume` "/Game/Sound/SoundClasses/Mix_Master.Mix_Master" "/Game/Sound/SoundClasses/Master.Master" (`/Game/Blueprints/SaveObjects/BP_AudioSettings.MasterVolume` _savegame_audiosettings))
  (`self.SetVolume` "/Game/Sound/SoundClasses/Mix_Master.Mix_Master" "/Game/Sound/SoundClasses/Music.Music" (`/Game/Blueprints/SaveObjects/BP_AudioSettings.MusicVolume` _savegame_audiosettings))
  (`self.SetVolume` "/Game/Sound/SoundClasses/Mix_Master.Mix_Master" "/Game/Sound/SoundClasses/Environment.Environment" (`/Game/Blueprints/SaveObjects/BP_AudioSettings.EnvironmentVolume` _savegame_audiosettings))
  (`self.SetVolume` "/Game/Sound/SoundClasses/Mix_Master.Mix_Master" "/Game/Sound/SoundClasses/SFX.SFX" (`/Game/Blueprints/SaveObjects/BP_AudioSettings.SFXVolume` _savegame_audiosettings))
  (`self.SetVolume` "/Game/Sound/SoundClasses/Mix_Master.Mix_Master" "/Game/Sound/SoundClasses/UI.UI" (`/Game/Blueprints/SaveObjects/BP_AudioSettings.UIVolume` _savegame_audiosettings)))

(fn `LoadAllSaves`
  (`self.LoadAudioSettings`)
  (`self.LoadHighScore`))

(fn `LoadAudioSettings`
  (bind _returnvalue (`GameplayStatics.DoesSaveGameExist` (`self.SaveSlot_AudioSettings`)))
  (if _returnvalue
    (bind _returnvalue_2 (`GameplayStatics.LoadGameFromSlot` (`self.SaveSlot_AudioSettings`)))
    (bind _asbp_audio_settings (cast `/Game/Blueprints/SaveObjects/BP_AudioSettings` _returnvalue_2))
    (set `self.SaveGame_AudioSettings` _asbp_audio_settings)
    (else
      (bind _returnvalue_3 (`GameplayStatics.CreateSaveGameObject` "/Game/Blueprints/SaveObjects/BP_AudioSettings.BP_AudioSettings_C"))
      (set `self.SaveGame_AudioSettings` _returnvalue_3))))

(fn `LoadHighScore`
  (bind _returnvalue (`GameplayStatics.DoesSaveGameExist` (`self.SaveSlot_HighScore`)))
  (if _returnvalue
    (bind _returnvalue_2 (`GameplayStatics.LoadGameFromSlot` (`self.SaveSlot_HighScore`)))
    (bind _asbp_high_score (cast `/Game/Blueprints/SaveObjects/BP_HighScore` _returnvalue_2))
    (set `self.SaveGame_HighScore` _asbp_high_score)
    (else
      (bind _returnvalue_3 (`GameplayStatics.CreateSaveGameObject` "/Game/Blueprints/SaveObjects/BP_HighScore.BP_HighScore_C"))
      (set `self.SaveGame_HighScore` _returnvalue_3))))

(fn `SaveAudioSettings`
  (`GameplayStatics.SaveGameToSlot` (`self.SaveGame_AudioSettings`) (`self.SaveSlot_AudioSettings`)))

(fn `SaveHighScore`
  (params (NewScore :type Integer))
  (set `/Game/Blueprints/SaveObjects/BP_HighScore.HighScore` NewScore (`self.SaveGame_HighScore`))
  (`GameplayStatics.SaveGameToSlot` (`self.SaveGame_HighScore`) (`self.SaveSlot_HighScore`)))

(fn `SetVolume`
  (params (Mix :type "SoundMix Object Reference") (Class :type "SoundClass Object Reference") (Value :type "Float (double-precision)"))
  (`GameplayStatics.SetBaseSoundMix` Mix)
  (`GameplayStatics.SetSoundMixClassOverride` Mix Class Value 1.0 0.0))