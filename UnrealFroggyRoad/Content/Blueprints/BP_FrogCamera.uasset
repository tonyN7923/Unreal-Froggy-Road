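; BP_FrogCamera is a follow camera actor that tracks the BP_Frog found in the level at BeginPlay.
; Each Tick it calls MoveTo, which uses VInterpTo to ease its location toward the frog's position plus CameraOffset.
; Stop restricts following to the X axis, holding the current Y and Z, and Enable restores following on all three axes.
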(event `self.ReceiveBeginPlay`
  (bind _returnvalue (`GameplayStatics.GetActorOfClass` "/Game/Blueprints/Animals/BP_Frog.BP_Frog_C"))
  (set `self.Frog` _returnvalue))

(event `self.ReceiveTick`
  (params (DeltaSeconds :type "Float (single-precision)"))
  (`self.Frog`
    (:`then`
      (if (`self.IsStopped`)
        (`self.MoveTo` (`KismetMathLibrary.MakeVector` (.x (+ (`self.K2_GetActorLocation` (`self.Frog`)) (`self.CameraOffset`))) (.y (`self.K2_GetActorLocation`)) (.z (`self.K2_GetActorLocation`))))
        (else
          (`self.MoveTo` (+ (`self.K2_GetActorLocation` (`self.Frog`)) (`self.CameraOffset`))))))
    (:`else`)))

(fn `Enable`
  (set `self.IsStopped` false))

(fn `MoveTo`
  (params (Target :type "Vector Structure"))
  (`self.K2_SetActorLocationAndRotation` (`KismetMathLibrary.VInterpTo` (`self.K2_GetActorLocation`) Target (`GameplayStatics.GetWorldDeltaSeconds`) 5.0)))

(fn `Stop`
  (set `self.IsStopped` true))

(fn `UserConstructionScript`)