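; BP_PlayerInput handles the Pause input action, toggling game pause and the WBP_PauseMenu widget.
; The current paused state selects the branch on each press.
; Pausing creates a new menu, shows the cursor and sets Game And UI input mode.
; Unpausing finds top-level menu widgets by class instead of a stored reference, removes them, hides the cursor and restores game-only input.
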(event `InputAction|Pause` :paused true
  (params (Key :type "Key Structure"))
  (bind _returnvalue (`GameplayStatics.GetPlayerController` 0))
  (bind _returnvalue_2 (`GameplayStatics.GetPlayerController` 0))
  (:`Pressed`
    (if (`GameplayStatics.IsGamePaused`)
      (bind _foundwidgets (`WidgetBlueprintLibrary.GetAllWidgetsOfClass` "/Game/Blueprints/Widgets/WBP_PauseMenu.WBP_PauseMenu_C"))
      (for _array_element _foundwidgets
        (`Widget.RemoveFromParent` _array_element))
      (`WidgetBlueprintLibrary.SetInputMode_GameOnly` _returnvalue_2)
      (set `PlayerController.bShowMouseCursor` false _returnvalue_2)
      (`GameplayStatics.SetGamePaused` false)
      (else
        (bind _returnvalue_3 (`|CreateWidget` "/Game/Blueprints/Widgets/WBP_PauseMenu.WBP_PauseMenu_C"))
        (`UserWidget.AddToViewport` _returnvalue_3 0)
        (set `PlayerController.bShowMouseCursor` true _returnvalue)
        (`WidgetBlueprintLibrary.SetInputMode_GameAndUIEx` _returnvalue null)
        (`GameplayStatics.SetGamePaused` true)))))