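; Platform item spawner for the Froggy Road game that spawns one randomly chosen item from its Items list on BeginPlay.
; Direction selects a stationary item at Y zero or one moving left or right, rotated to match and starting at the opposite game mode spawn bound.
; Moving items receive the far bound as their kill Y, and all items receive the spawner's Speed.
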(event `self.ReceiveBeginPlay`
  (bind _returnvalue (`GameplayStatics.GetActorOfClass` "/Game/Blueprints/BP_FroggyRoadGameMode.BP_FroggyRoadGameMode_C"))
  (set `self.GameMode` _returnvalue)
  (`self.SpawnItem`))

(fn `SpawnItem`
  (switch `/Game/Data/E_PlatformDirection` (`self.Direction`)
    (:`NewEnumerator0`
      (`|SpawnActorFromClass` (`KismetArrayLibrary.Array_Random` (`self.Items`)) (`self.CreateItemTransform` (struct)) "Undefined" "OverrideRootScale" null (`self.Speed`) 0.0 false null))
    (:`NewEnumerator1`
      (bind (_vector _rotator) (`/Game/Blueprints/BP_TransformUtility.GetLeftVectorAndRotator`))
      (`|SpawnActorFromClass` (`KismetArrayLibrary.Array_Random` (`self.Items`)) (`self.CreateItemTransform` _rotator (`/Game/Blueprints/BP_FroggyRoadGameMode.RightSpawnBound` (`self.GameMode`))) "Undefined" "OverrideRootScale" null (`self.Speed`) (`/Game/Blueprints/BP_FroggyRoadGameMode.LeftSpawnBound` (`self.GameMode`)) true null))
    (:`NewEnumerator2`
      (bind (_vector_2 _rotator_2) (`/Game/Blueprints/BP_TransformUtility.GetRightVectorAndRotator`))
      (`|SpawnActorFromClass` (`KismetArrayLibrary.Array_Random` (`self.Items`)) (`self.CreateItemTransform` _rotator_2 (`/Game/Blueprints/BP_FroggyRoadGameMode.LeftSpawnBound` (`self.GameMode`))) "Undefined" "OverrideRootScale" null (`self.Speed`) (`/Game/Blueprints/BP_FroggyRoadGameMode.RightSpawnBound` (`self.GameMode`)) true null))))

(fn `UserConstructionScript`)