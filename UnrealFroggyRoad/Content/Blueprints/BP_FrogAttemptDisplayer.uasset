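; BP_FrogAttemptDisplayer is an actor that shows remaining attempts as three frog meshes.
; On BeginPlay its SceneCaptureComponent2D is limited to its own components, and the frogs are gathered into an array with a counter set to its length.
; DeductAttempt decrements the counter and sets IsDead on that frog's ABP_Frog anim instance, killing frogs from last to first.
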(event `self.ReceiveBeginPlay`
  (`SceneCaptureComponent.ShowOnlyActorComponents` (`self.SceneCaptureComponent2D`) self false)
  (bind _output_get (set `self.Frogs` (`|MakeArray` (`self.Frog`) (`self.Frog1`) (`self.Frog2`))))
  (set `self.LastFrogDead` (`KismetArrayLibrary.Array_Length` _output_get)))

(fn `DeductAttempt`
  (bind _result (`/Engine/EditorBlueprintResources/StandardMacros.DecrementInt` (`self.LastFrogDead`))
    (:`  `
      (bind _asabp_frog (cast `/Game/Blueprints/Animals/ABP_Frog` (`SkeletalMeshComponent.GetAnimInstance` (`|GetArrayItem` (`self.Frogs`) _result))))
      (set `/Game/Blueprints/Animals/ABP_Frog.IsDead` true _asabp_frog))))

(fn `UserConstructionScript`)