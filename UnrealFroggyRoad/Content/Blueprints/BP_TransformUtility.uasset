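; BP_TransformUtility is a set of helper functions that supply standard directions and rotations.
; Four functions return the forward, backward, left or right vector of a zero rotation, so fixed world axes, each paired with a rotator built from that vector.
; Backward and left negate the forward and right vectors.
; GetRandomRotationZ returns a rotator with random yaw over a full turn and no pitch or roll.
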(fn `GetBackwardVectorAndRotator`
  (returns (Vector :type "Vector Structure") (Rotator :type "Rotator Structure"))
  (bind _returnvalue (`KismetMathLibrary.NegateVector` (`KismetMathLibrary.GetForwardVector` (struct))))
  (return _returnvalue (`KismetMathLibrary.Conv_VectorToRotator` _returnvalue)))

(fn `GetForwardVectorAndRotator`
  (returns (Vector :type "Vector Structure") (Rotator :type "Rotator Structure"))
  (bind _returnvalue (`KismetMathLibrary.GetForwardVector` (struct)))
  (return _returnvalue (`KismetMathLibrary.Conv_VectorToRotator` _returnvalue)))

(fn `GetLeftVectorAndRotator`
  (returns (Vector :type "Vector Structure") (Rotator :type "Rotator Structure"))
  (bind _returnvalue (`KismetMathLibrary.NegateVector` (`KismetMathLibrary.GetRightVector` (struct))))
  (return _returnvalue (`KismetMathLibrary.Conv_VectorToRotator` _returnvalue)))

(fn `GetRandomRotationZ`
  (returns (Rotator :type "Rotator Structure"))
  (return (`KismetMathLibrary.MakeRotator` 0.0 0.0 (`KismetMathLibrary.RandomFloatInRange` 0.0 360.0))))

(fn `GetRightVectorAndRotator`
  (returns (Vector :type "Vector Structure") (Rotator :type "Rotator Structure"))
  (bind _returnvalue (`KismetMathLibrary.GetRightVector` (struct)))
  (return _returnvalue (`KismetMathLibrary.Conv_VectorToRotator` _returnvalue)))