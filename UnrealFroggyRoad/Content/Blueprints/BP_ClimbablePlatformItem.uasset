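; BP_ClimbablePlatformItem is a climbable platform that reports the climb spot closest to a given position.
; Climb spots are the direct child components of its ClimbSpots component.
; GetNearestClimbSpot loops over them, comparing world-space distance against a running SpotDistance value, and returns the nearest match.
; The construction script only calls its parent.
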(fn `GetNearestClimbSpot`
  (params (CurrentPosition :type "Vector Structure"))
  (returns (Spot :type "SceneComponent Object Reference"))
  (locals (NearestSpot :type "SceneComponent Object Reference") (SpotDistance :type "Float (double-precision)" :default 9999.0))
  (for _array_element (`SceneComponent.GetChildrenComponents` (`self.ClimbSpots`) false)
    (bind _returnvalue (`KismetMathLibrary.Vector_Distance` (`SceneComponent.K2_GetComponentLocation` _array_element) (`local.CurrentPosition`)))
    (if (< _returnvalue (`local.SpotDistance`))
      (set `local.SpotDistance` _returnvalue)
      (set `local.NearestSpot` _array_element)))
  (return (`local.NearestSpot`)))

(fn `UserConstructionScript`
  (`parent.UserConstructionScript`))